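; Status_AttributePlus generates a random attribute bonus stored in a Status value when play begins.
; It rolls a rarity, zeroes Status, then makes one fewer random attribute picks than the rarity.
; Health and attack speed scale from random levels bounded by squared rarity, with repeat picks overwriting earlier values.
; The attack power branch discards its roll and writes zero, and a fourth outcome changes nothing.
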(event EventBeginPlay
  (CallFunction|GetBaseRarity)
  (Default|Initialize (Variables|Default|Getstatus) 0.0 0.0 0.0 0.0)
  (CallFunction|GetAttributes))

(event EventTick
  (params (DeltaSeconds :type Float%20%28single-precision%29)))

(fn DecideRarityLevel
  (bind _rarity (Variables|Default|Getrarity))
  (return (Math|Random|RandomIntegerinRange (Math|Float|Round (Math|Float|Square (Math|Conversions|ToFloat(Integer) (- _rarity 1)))) (Math|Float|Round (Math|Float|Square (Math|Conversions|ToFloat(Integer) _rarity))))))

(fn GetBaseRarity
  (Variables|Default|Setrarity (Math|Random|RandomIntegerinRange 2 5)))

(fn GetAttributes
  (bind _status (Variables|Default|Getstatus))
  (for _index (range 1 (- (Variables|Default|Getrarity) 1))
    (switch int (Math|Random|RandomInteger 4)
      (:0
        (bind _raritylevel (CallFunction|DecideRarityLevel))
        (Variables|/Game/Blueprints/Stats/StatusProfile.StatusProfile_C|SetHealth _status (Math|Conversions|ToFloat(Integer) (* _raritylevel 10))))
      (:1
        (CallFunction|DecideRarityLevel)
        (Variables|/Game/Blueprints/Stats/StatusProfile.StatusProfile_C|SetAttackPowerLowerLimit _status (Math|Conversions|ToFloat(Integer) (* 0 3)))
        (Variables|/Game/Blueprints/Stats/StatusProfile.StatusProfile_C|SetAttackPowerUpperLimit _status 0.0))
      (:2
        (bind _raritylevel_2 (CallFunction|DecideRarityLevel))
        (Variables|/Game/Blueprints/Stats/StatusProfile.StatusProfile_C|SetAttackSpeed _status (/ (Math|Conversions|ToFloat(Integer) _raritylevel_2) 1e+02))))))