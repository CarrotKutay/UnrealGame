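; StatusProfile is a stats Blueprint with attack power limits, health and attack speed.
; GetAttackPower is meant to roll a random value between the limits, but its entry is unwired and the roll is unused.
; Add is meant to combine two profiles, but as written it doubles those four stats on the valid profile passed in, reading none of its own values.
; BeginPlay and Tick are empty.
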(event EventBeginPlay)

(event EventTick
  (params (DeltaSeconds :type Float%20%28single-precision%29)))

(fn GetAttackPower
  ;[1 1 1 0] get random value between upper and lower boudn as attack range
)

(fn Add
  (params (StatusProfile :type Status%20Profile%20Object%20Reference))
  ;[1 1 1 0] add a status to another status return void
  (bind _statusprofile (LocalVariables|GetStatusProfile)
    (:then
      (Variables|StatusProfile_C|SetAttackPowerLowerLimit StatusProfile (+ (Variables|StatusProfile_C|GetAttackPowerLowerLimit _statusprofile) (Variables|StatusProfile_C|GetAttackPowerLowerLimit StatusProfile)))
      (Variables|StatusProfile_C|SetAttackPowerUpperLimit StatusProfile (+ (Variables|StatusProfile_C|GetAttackPowerUpperLimit StatusProfile) (Variables|StatusProfile_C|GetAttackPowerUpperLimit _statusprofile)))
      (Variables|StatusProfile_C|SetHealth StatusProfile (+ (Variables|StatusProfile_C|GetHealth _statusprofile) (Variables|StatusProfile_C|GetHealth StatusProfile)))
      (Variables|StatusProfile_C|SetAttackSpeed StatusProfile (+ (Variables|StatusProfile_C|GetAttackSpeed StatusProfile) (Variables|StatusProfile_C|GetAttackSpeed _statusprofile)))
      (return))
    (:else
      (return))))