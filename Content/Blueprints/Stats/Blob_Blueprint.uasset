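; A stat blob pickup actor that passes its Attributes to the StatusPlayer component of the actor overlapping it.
; BeginPlay tints the mesh with the Attributes color material.
; On overlap, a TargetReached while loop starts an eased MoveComponentTo toward that actor; both loop exit and move completion add the status and destroy the blob.
; The distance check that would update TargetReached and stop the move is disconnected.
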(event EventBeginPlay
  (Rendering|Material|SetMaterial (Variables|Debug|GetStaticMeshComponent) 0 (Variables|/Game/Blueprints/Stats/Status_AttributePlus.Status_AttributePlus_C|Getcolor (Variables|Default|GetAttributes))))

(event Collision|EventActorBeginOverlap
  (params (OtherActor :type Actor%20Object%20Reference))
  (while (Variables|Default|GettargetReached)
    (Components|MoveComponentTo (Variables|Debug|GetStaticMeshComponent) (Transformation|GetActorLocation OtherActor) (Transformation|GetActorRotation OtherActor) true true 0.8 false)
    (Default|AddStatus (Actor|GetComponentbyClass OtherActor "/Game/Blueprints/Stats/StatusPlayer.StatusPlayer_C") (Variables|Default|GetAttributes))
    (Actor|DestroyActor))
  (Default|AddStatus (Actor|GetComponentbyClass OtherActor "/Game/Blueprints/Stats/StatusPlayer.StatusPlayer_C") (Variables|Default|GetAttributes))
  (Actor|DestroyActor))

(event EventTick
  (params (DeltaSeconds :type Float%20%28single-precision%29)))

(fn ConstructionScript)