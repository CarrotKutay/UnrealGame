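; Enemy character Blueprint that deals periodic damage to the player's StatusPlayer component and tints its own body.
; Begin overlap casts the overlapping actor itself to PlayerController, then caches the controlled pawn's status component and starts a looping one-second DamageHero timer.
; Each tick truncates CurrentHealth and subtracts Damage; any end overlap clears the timer.
; The construction script applies EnemyColor through a dynamic material instance.
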(event Custom|DamageHero
  (bind _playerstatus (Variables|Default|GetPlayerStatus))
  (Variables|/Game/Blueprints/Stats/StatusProfile.StatusProfile_C|SetCurrentHealth _playerstatus (Math|Conversions|ToFloat(Integer) (- (Math|Float|Truncate (Variables|/Game/Blueprints/Stats/StatusProfile.StatusProfile_C|GetCurrentHealth _playerstatus)) (Variables|Default|GetDamage)))))

(event Collision|EventActorBeginOverlap
  (params (OtherActor :type Actor%20Object%20Reference))
  (bind _asplayer_controller (Utilities|Casting|CastToPlayerController OtherActor))
  (Utilities|IsValid (Actor|GetComponentbyClass (Pawn|GetControlledPawn _asplayer_controller) "/Game/Blueprints/Stats/StatusPlayer.StatusPlayer_C")
    (:Is%20Valid
      (Variables|Default|SetPlayerStatus (Actor|GetComponentbyClass (Pawn|GetControlledPawn _asplayer_controller) "/Game/Blueprints/Stats/StatusPlayer.StatusPlayer_C"))
      (Utilities|Time|SetTimerbyFunctionName 0 "DamageHero" 1.0 true))))

(event Collision|EventActorEndOverlap
  (params (OtherActor :type Actor%20Object%20Reference))
  (if true
    (Utilities|Time|ClearTimerbyFunctionName 0 "DamageHero")))

(fn ConstructionScript
  (bind _returnvalue (Rendering|Material|CreateDynamicMaterialInstance (Variables|Character|GetMesh) 0 0 "None" :!class /Script/Engine.PrimitiveComponent))
  (bind _output_get (Variables|Default|SetDynamicMat _returnvalue))
  (Rendering|Material|SetVectorParameterValue _output_get "BodyColor" (Variables|Default|GetEnemyColor) :!class /Script/Engine.MaterialInstanceDynamic))