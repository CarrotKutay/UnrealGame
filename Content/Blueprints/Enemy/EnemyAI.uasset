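; EnemyAI is an enemy AI controller Blueprint that makes its controlled pawn chase the nearer of two players.
; BeginPlay starts a looping one-second timer that calls FollowPlayer by name.
; FollowPlayer compares the pawn's distance to player characters 0 and 1, then issues AIMoveTo toward the closer one, choosing player 1 on a tie.
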(event Custom|FollowPlayer
  (bind _returnvalue (Pawn|GetControlledPawn))
  (bind _returnvalue_2 (Pawn|GetControlledPawn))
  (if (< (Transformation|GetDistanceTo _returnvalue (Game|GetPlayerCharacter 0)) (Transformation|GetDistanceTo _returnvalue (Game|GetPlayerCharacter 1)))
    (AI|AIMoveTo _returnvalue_2 "0, 0, 0" (Game|GetPlayerCharacter 0) 5.0 false)
    (else
      (AI|AIMoveTo _returnvalue_2 "0, 0, 0" (Game|GetPlayerCharacter 1) 5.0 false))))

(event EventBeginPlay
  (Utilities|Time|SetTimerbyFunctionName 0 "FOllowPlayer" 1.0 true))

(fn ConstructionScript)